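; Phone child Blueprint that shakes as if ringing and can show a phone clue to the player.
; While not Used, Tick alternates a local roll rotation behind a short Delay to fake the ringing.
; BeginPlay runs the parent logic and binds CheckDrawer to the player's special interact, which opens the PhoneClue widget when the player is in range and NumPlanes is two.
; Delayed ring start and held-item setup nodes are left disconnected.
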(event `self.ReceiveTick`
  (params (DeltaSeconds :type "Float (single-precision)"))
  ;[1 1 1] Phone Ringing Script
  (if (not (`self.Used`))
    (`KismetSystemLibrary.Delay` 0.2)
    (bind _output_get (set `self.rotation` (* (`self.rotation`) -1.0)))
    (`self.K2_AddActorLocalRotation` (`KismetMathLibrary.MakeRotator` _output_get))))

(event `self.ReceiveBeginPlay`
  (`parent.ReceiveBeginPlay`)
  (add `/Game/Blueprints/PlayerBP.SpecialInteract` (`self.Player`) (delegate `Check Drawer`)))

(event `Check Drawer`
  (if (and (`self.PlayerInRange`) (== (`self.NumPlanes`) 2))
    (bind _returnvalue (`|CreateWidget` "/Game/Blueprints/UI/PhoneClue.PhoneClue_C"))
    (`UserWidget.AddToViewport` _returnvalue 0)))

(fn `UserConstructionScript`
  (`parent.UserConstructionScript`))