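; Child fan Blueprint that the player can switch on and off with the special interact input while in range.
; It binds that input on BeginPlay, then flips FanOn and calls FanToggled, only when NumPlanes is exactly 2.
; Capsule overlaps extend the parent's handling, showing an on/off prompt matching the current state on entry and removing it on exit.
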(event `self.ReceiveBeginPlay`
  (`parent.ReceiveBeginPlay`)
  (add `/Game/Blueprints/PlayerBP.SpecialInteract` (`self.Player`) (delegate `Check Drawer`)))

(event `Check Drawer`
  (if (and (`self.PlayerInRange`) (== (`self.NumPlanes`) 2))
    (set `self.fanOn` (not (`self.fanOn`)))
    (`self.FanToggled`)))

(event `self.Capsule.OnComponentBeginOverlap`
  (params (OverlappedComponent :type "PrimitiveComponent Object Reference") (OtherActor :type "Actor Object Reference") (OtherComp :type "PrimitiveComponent Object Reference") (OtherBodyIndex :type Integer) (bFromSweep :type Boolean) (SweepResult :type "HitResult Structure (by ref)"))
  (bind _fantoggleui (`self.fanToggleUI`))
  (bind _fantoggleui_2 (`self.fanToggleUI`))
  ;[0 0 0] Interaction Prompt Display Based On Proximity
  (`self.Parent Begin Overlap` OtherActor)
  ;[1 1 1] Fan UI
  (if (== (`self.NumPlanes`) 2)
    (if (`self.fanOn`)
      (`/Engine/EditorBlueprintResources/StandardMacros.IsValid` _fantoggleui_2
        (:`Is Valid`
          (`Widget.RemoveFromParent` _fantoggleui_2))
        (:`Is Not Valid`
          _))
      (bind _returnvalue (`self.Create Special Interact Prompt` _fantoggleui_2 "Press I to Turn Fan Off"))
      (set `self.fanToggleUI` _returnvalue)
      (else
        (`/Engine/EditorBlueprintResources/StandardMacros.IsValid` _fantoggleui
          (:`Is Valid`
            (`Widget.RemoveFromParent` _fantoggleui))
          (:`Is Not Valid`
            _))
        (bind _returnvalue_2 (`self.Create Special Interact Prompt` _fantoggleui "Press I to Turn Fan On"))
        (set `self.fanToggleUI` _returnvalue_2)))))

(event `self.Capsule.OnComponentEndOverlap`
  (params (OverlappedComponent :type "PrimitiveComponent Object Reference") (OtherActor :type "Actor Object Reference") (OtherComp :type "PrimitiveComponent Object Reference") (OtherBodyIndex :type Integer))
  ;[0 0 0] Interaction Prompt Display Based On Proximity
  (`self.Parent End Overlap` OtherActor)
  ;[1 1 1] Fan UI
  (`self.Delete Special Interact Prompt` (`self.fanToggleUI`))
  (set `self.fanToggleUI` null))

(fn `UserConstructionScript`
  (`parent.UserConstructionScript`))