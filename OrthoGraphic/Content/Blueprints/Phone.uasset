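; Phone actor that shakes as if ringing until the player interacts with it, then gets knocked loose and disappears.
; Tick flips a roll offset through short delays while unused, and a looping ten-second BeginPlay timer rebinds the interact event and resets the shake.
; Box1 overlaps track player range and swap the prompt and knife-count widgets.
; In-range interaction enables physics on Receiver and Box, pushes them, then destroys the actor.
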(event `self.ReceiveBeginPlay`
  ;[1 1 1] Phone Ringing Script
  (add `/Game/Blueprints/PlayerBP.InteractEvent` (`self.Player`) (delegate `HandleInteraction`) :!label _label)
  (`KismetSystemLibrary.Delay` 10.0)
  (set `self.Used` false)
  (set `self.rotation` 30.0)
  (`self.K2_AddActorLocalRotation` (`KismetMathLibrary.MakeRotator` 15.0))
  (goto _label))

(event `self.ReceiveTick`
  (params (DeltaSeconds :type "Float (single-precision)"))
  ;[1 1 1] Phone Ringing Script
  (if (not (`self.Used`))
    (`KismetSystemLibrary.Delay` 0.2)
    (bind _output_get (set `self.rotation` (* (`self.rotation`) -1.0)))
    (`self.K2_AddActorLocalRotation` (`KismetMathLibrary.MakeRotator` _output_get))))

(event `self.Box1.OnComponentBeginOverlap`
  (params (OverlappedComponent :type "PrimitiveComponent Object Reference") (OtherActor :type "Actor Object Reference") (OtherComp :type "PrimitiveComponent Object Reference") (OtherBodyIndex :type Integer) (bFromSweep :type Boolean) (SweepResult :type "HitResult Structure (by ref)"))
  ;[1 1 1] Interaction Prompt Display Based On Proximity
  (cast `/Game/Blueprints/PlayerBP` OtherActor)
  (set `self.PlayerInRange` true)
  (bind _returnvalue (`|CreateWidget` "/Game/Blueprints/UI/Interact_prompt.Interact_prompt_C"))
  (`UserWidget.AddToViewport` _returnvalue 0))

(event `self.Box1.OnComponentEndOverlap`
  (params (OverlappedComponent :type "PrimitiveComponent Object Reference") (OtherActor :type "Actor Object Reference") (OtherComp :type "PrimitiveComponent Object Reference") (OtherBodyIndex :type Integer))
  ;[1 1 1] Interaction Prompt Display Based On Proximity
  (cast `/Game/Blueprints/PlayerBP` OtherActor)
  (set `self.PlayerInRange` false)
  (`WidgetLayoutLibrary.RemoveAllWidgets`)
  (bind _returnvalue (`|CreateWidget` "/Game/Blueprints/UI/Knife_count.Knife_count_C"))
  (`UserWidget.AddToViewport` _returnvalue 0))

(event `HandleInteraction`
  (bind _receiver (`self.Receiver`))
  ;[1 1 1] Interaction Code Body
  (if (`self.PlayerInRange`)
    (`PrimitiveComponent.SetSimulatePhysics` _receiver true)
    (`PrimitiveComponent.SetSimulatePhysics` (`self.Box`) true)
    (set `self.Used` true)
    (`PrimitiveComponent.AddForce` _receiver (`KismetMathLibrary.MakeVector` 100.0) "None" true)
    (`PrimitiveComponent.AddForce` (`self.Box`) (`KismetMathLibrary.MakeVector` 100.0) "None" true)
    (`KismetSystemLibrary.Delay` 2.0)
    (`self.K2_DestroyActor`)))

(fn `UserConstructionScript`)