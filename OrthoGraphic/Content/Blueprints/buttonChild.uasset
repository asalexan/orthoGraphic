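; Child button Blueprint that lets the player toggle a button on or off with a special interact input.
; BeginPlay binds FlipSwitch to the player's special interact event, which flips ButtonOn and calls CallButtonToggled only while the player is in range and NumPlanes is two.
; Capsule overlaps extend the parent's handling to create, update or delete the on-screen toggle prompt.
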(event `self.ReceiveBeginPlay`
  (`parent.ReceiveBeginPlay`)
  (add `/Game/Blueprints/PlayerBP.SpecialInteract` (`self.Player`) (delegate `FlipSwitch`)))

(event `FlipSwitch`
  (if (and (`self.PlayerInRange`) (== (`self.NumPlanes`) 2))
    (set `self.buttonOn` (not (`self.buttonOn`)))
    (`self.ButtonToggled`)))

(event `self.Capsule.OnComponentBeginOverlap`
  (params (OverlappedComponent :type "PrimitiveComponent Object Reference") (OtherActor :type "Actor Object Reference") (OtherComp :type "PrimitiveComponent Object Reference") (OtherBodyIndex :type Integer) (bFromSweep :type Boolean) (SweepResult :type "HitResult Structure (by ref)"))
  (bind _buttononprompt (`self.buttonOnPrompt`))
  (bind _interact_text (`/Game/Blueprints/UI/SpecialInteract_prompt.Interact_Text` (`self.buttonOnPrompt`)))
  (`self.Parent Begin Overlap` OtherActor)
  ;[0 0 0] Button UI
  (if (== (`self.NumPlanes`) 2)
    (`/Engine/EditorBlueprintResources/StandardMacros.IsValid` _buttononprompt
      (:`Is Valid`
        (if (`self.buttonOn`)
          (`TextBlock.SetText` _interact_text "Press I to Turn Button Off")
          (else
            (`TextBlock.SetText` _interact_text "Press I to Turn Button On"))))
      (:`Is Not Valid`
        (bind _returnvalue (`self.Create Special Interact Prompt` _buttononprompt "Press I to Turn Button On"))
        (set `self.buttonOnPrompt` _returnvalue)))))

(event `self.Capsule.OnComponentEndOverlap`
  (params (OverlappedComponent :type "PrimitiveComponent Object Reference") (OtherActor :type "Actor Object Reference") (OtherComp :type "PrimitiveComponent Object Reference") (OtherBodyIndex :type Integer))
  (`self.Parent End Overlap` OtherActor)
  ;[0 0 0] Button UI
  (`self.Delete Special Interact Prompt` (`self.buttonOnPrompt`))
  (set `self.buttonOnPrompt` null))

(fn `UserConstructionScript`
  (`parent.UserConstructionScript`))