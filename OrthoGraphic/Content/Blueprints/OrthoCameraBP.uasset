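; Orthographic camera Blueprint that orbits the scene in 90-degree steps on the Spin Left and Spin Right inputs.
; Each press rotates the actor's forward vector around world Z to set the new rotation, then places it 150 units back along that direction, facing the world origin.
; The move is instant, and each spin ends with CallLockHideUnhide.
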(event `InputAction|Spin Left`
  (params (Key :type "Key Structure"))
  (bind _returnvalue (`KismetMathLibrary.Conv_VectorToRotator` (`KismetMathLibrary.RotateAngleAxis` (`KismetMathLibrary.Conv_RotatorToVector` (`self.K2_GetActorRotation`)) -90.0 (0.0 0.0 1.0))))
  ;[0 0 0] Spin Camera Left
  (:`Pressed`
    (`self.K2_SetActorLocationAndRotation` (* (`KismetMathLibrary.Normal` (`KismetMathLibrary.GetForwardVector` _returnvalue)) -150.0) _returnvalue)
    (`self.Lock Hide/Unhide`)))

(event `InputAction|Spin Right`
  (params (Key :type "Key Structure"))
  (bind _returnvalue (`KismetMathLibrary.Conv_VectorToRotator` (`KismetMathLibrary.RotateAngleAxis` (`KismetMathLibrary.Conv_RotatorToVector` (`self.K2_GetActorRotation`)) 90.0 (0.0 0.0 1.0))))
  ;[0 0 0] Spin Camera Right
  (:`Pressed`
    (`self.K2_SetActorLocationAndRotation` (* (`KismetMathLibrary.Normal` (`KismetMathLibrary.GetForwardVector` _returnvalue)) -150.0) _returnvalue)
    (`self.Lock Hide/Unhide`)))

(fn `UserConstructionScript`)