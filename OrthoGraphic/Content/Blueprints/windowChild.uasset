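; Child interactable Blueprint for a window the player can knock on once, using a special interact prompt.
; Capsule overlaps extend parent range handling to show or remove the knock prompt while the window is interactable.
; The player's special interact event steps Plane1 through timed material frames, swaps its stored normal and selected materials, then disables interaction.
; When Animated is set, a Delay-throttled Tick also loops four frame materials as a flipbook.
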(event `self.ReceiveBeginPlay`
  (`parent.ReceiveBeginPlay`)
  (add `/Game/Blueprints/PlayerBP.SpecialInteract` (`self.Player`) (delegate `Window Interact Event`)))

(event `Window Interact Event`
  (bind _plane1 (`self.Plane1`))
  (if (and (`self.Interactable`) (`self.PlayerInRange`))
    (`PrimitiveComponent.SetMaterial` _plane1 0 (`self.anim_frame2`))
    (`KismetSystemLibrary.Delay` 0.5)
    (`PrimitiveComponent.SetMaterial` _plane1 0 (`self.anim_frame3`))
    (`KismetSystemLibrary.Delay` 0.5)
    (`PrimitiveComponent.SetMaterial` _plane1 0 (`self.anim_frame4`))
    (`KismetSystemLibrary.Delay` 0.5)
    (`PrimitiveComponent.SetMaterial` _plane1 0 (`self.anim_frame1`))
    (set `self.plane1_mat` "/Game/Materials/Window/windowMat.windowMat")
    (set `self.plane1_selectedMat` "/Game/Materials/Window/window_selectedMat.window_selectedMat")
    (set `self.Interactable` false)
    (`self.Delete Special Interact Prompt` (`self.knockOnWindowUI`))
    (set `self.knockOnWindowUI` null)))

(event `self.Capsule.OnComponentBeginOverlap`
  (params (OverlappedComponent :type "PrimitiveComponent Object Reference") (OtherActor :type "Actor Object Reference") (OtherComp :type "PrimitiveComponent Object Reference") (OtherBodyIndex :type Integer) (bFromSweep :type Boolean) (SweepResult :type "HitResult Structure (by ref)"))
  (bind _interactable (`self.Interactable`))
  (`self.Parent Begin Overlap` OtherActor _interactable)
  (if (and _interactable (`self.PlayerInRange`))
    (bind _returnvalue (`self.Create Special Interact Prompt` (`self.knockOnWindowUI`) "Press I to Knock On Window"))
    (set `self.knockOnWindowUI` _returnvalue)))

(event `self.Capsule.OnComponentEndOverlap`
  (params (OverlappedComponent :type "PrimitiveComponent Object Reference") (OtherActor :type "Actor Object Reference") (OtherComp :type "PrimitiveComponent Object Reference") (OtherBodyIndex :type Integer))
  (`self.Parent End Overlap` OtherActor)
  (`self.Delete Special Interact Prompt` (`self.knockOnWindowUI`))
  (set `self.knockOnWindowUI` null))

(event `self.ReceiveTick`
  (params (DeltaSeconds :type "Float (single-precision)"))
  (`KismetSystemLibrary.Delay` 0.2)
  (if (`self.Animated`)
    (if (== (`self.curFrame`) 1)
      (set `self.curFrame` 2)
      (`PrimitiveComponent.SetMaterial` (`self.Plane1`) 0 (`self.anim_frame1`))
      (elif (== (`self.curFrame`) 2)
        (set `self.curFrame` 3)
        (`PrimitiveComponent.SetMaterial` (`self.Plane1`) 0 (`self.anim_frame2`))
        (elif (== (`self.curFrame`) 3)
          (set `self.curFrame` 4)
          (`PrimitiveComponent.SetMaterial` (`self.Plane1`) 0 (`self.anim_frame3`))
          (elif (== (`self.curFrame`) 4)
            (set `self.curFrame` 1)
            (`PrimitiveComponent.SetMaterial` (`self.Plane1`) 0 (`self.anim_frame4`))))))))

(fn `UserConstructionScript`
  (`parent.UserConstructionScript`))