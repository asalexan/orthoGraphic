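; 2PTable is an interactable actor Blueprint, apparently an unfinished copy of a shared interaction template.
; On BeginPlay it binds HandleInteraction to the Player's interact event, but the handler only checks PlayerInRange and does nothing.
; Proximity prompt widgets, range-flag updates, a phone-ringing delay, rotation and destroy logic are all disconnected, so none of them run.
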(event `self.ReceiveBeginPlay`
  (add `/Game/Blueprints/PlayerBP.InteractEvent` (`self.Player`) (delegate `HandleInteraction`)))

(event `HandleInteraction`
  ;[1 1 1] Interaction Code Body
  (if (`self.PlayerInRange`)
    _))

(fn `UserConstructionScript`)