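; Level 2 soft-lock checker that warns the player when too many button drawers have been collected.
; On BeginPlay it binds to the collected notification of two referenced ButtonDrawers and increments a counter each time one fires.
; Once the count reaches DrawerMin, it creates a SoftLockNotice widget and adds it to the viewport.
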(event `self.ReceiveBeginPlay`
  (add `/Game/Blueprints/drawerChild.DrawerCollectedNotif` (`self.ButtonDrawer`) (delegate `DrawerCount`))
  (add `/Game/Blueprints/drawerChild.DrawerCollectedNotif` (`self.ButtonDrawer2`) (delegate `DrawerCount`)))

(event `DrawerCount`
  (set `self.DrawersCollected` (+ (`self.DrawersCollected`) 1))
  (if (>= (`self.DrawersCollected`) (`self.DrawerMin`))
    (bind _returnvalue (`|CreateWidget` "/Game/Blueprints/UI/SoftLockNotice.SoftLockNotice_C"))
    (`UserWidget.AddToViewport` _returnvalue 0)))

(fn `UserConstructionScript`)