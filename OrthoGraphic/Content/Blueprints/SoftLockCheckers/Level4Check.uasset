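; Level 4 soft-lock checker that shows a SoftLockNotice widget when watched pickup events occur.
; On BeginPlay it binds to pickup notifications from a button and a fan, plus collected notifications from two button drawers and two fan drawers.
; Picking up the button or fan shows the notice immediately, while drawer collections increment a counter that shows it upon reaching DrawerMin.
; Each trigger creates a new widget, with no guard against duplicates.
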(event `FanPickedUp`
  (bind _returnvalue (`|CreateWidget` "/Game/Blueprints/UI/SoftLockNotice.SoftLockNotice_C" :!label _label))
  (`UserWidget.AddToViewport` _returnvalue 0))

(event `ButtonPickedUp`
  (goto _label))

(event `self.ReceiveBeginPlay`
  (add `/Game/Blueprints/drawerChild.DrawerCollectedNotif` (`self.ButtonDrawer2`) (delegate `DrawerCount`))
  (add `/Game/Blueprints/drawerChild.DrawerCollectedNotif` (`self.ButtonDrawer`) (delegate `DrawerCount`))
  (add `/Game/Blueprints/drawerChild.DrawerCollectedNotif` (`self.FanDrawer`) (delegate `DrawerCount`))
  (add `/Game/Blueprints/drawerChild.DrawerCollectedNotif` (`self.FanDrawer2`) (delegate `DrawerCount`))
  (add `/Game/Blueprints/buttonChild.ButtonPickedUpNotif` (`self.Button`) (delegate `ButtonPickedUp`))
  (add `/Game/Blueprints/fanChild.FanPickedUpNotif` (`self.Fan`) (delegate `FanPickedUp`)))

(event `DrawerCount`
  (set `self.DrawersCollected` (+ (`self.DrawersCollected`) 1))
  (if (>= (`self.DrawersCollected`) (`self.DrawerMin`))
    (goto _label)))

(fn `UserConstructionScript`)