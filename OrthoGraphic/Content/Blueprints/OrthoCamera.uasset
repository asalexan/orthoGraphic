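; Orthographic camera actor that snaps around the scene in 90-degree steps when the Player's spin left or right events fire.
; Each spin rotates its facing about world Z and places it DistanceFromScene from the world origin along that forward axis.
; It then calls LockHideUnhide and UpdateSort so the view's dependents can refresh; UpdateSort also fires at BeginPlay.
; Only the left spin updates ViewingAxis.
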(event `self.ReceiveBeginPlay`
  (bind _player (`self.Player`))
  (`self.updateSort`)
  (add `/Game/Blueprints/PlayerBP.SpinViewLeft` _player (delegate `SpinViewLeft`))
  (add `/Game/Blueprints/PlayerBP.SpinViewRight` _player (delegate `SpinViewRight`)))

(event `SpinViewLeft`
  (bind _returnvalue (`KismetMathLibrary.Conv_VectorToRotator` (`KismetMathLibrary.RotateAngleAxis` (`KismetMathLibrary.Conv_RotatorToVector` (`self.K2_GetActorRotation`)) -90.0 (0.0 0.0 1.0))))
  (`self.K2_SetActorLocationAndRotation` (* (`KismetMathLibrary.Normal` (`KismetMathLibrary.GetForwardVector` _returnvalue)) (`self.DistanceFromScene`)) _returnvalue)
  (set `self.ViewingAxis` (`KismetMathLibrary.GetForwardVector` (`SceneComponent.K2_GetComponentRotation` (`self.OrthoCamera`))))
  (`self.Lock Hide/Unhide`) ; Lock/unlock corresponding view
  (`self.updateSort`))

(event `SpinViewRight`
  (bind _returnvalue (`KismetMathLibrary.Conv_VectorToRotator` (`KismetMathLibrary.RotateAngleAxis` (`KismetMathLibrary.Conv_RotatorToVector` (`self.K2_GetActorRotation`)) 90.0 (0.0 0.0 1.0))))
  (`self.K2_SetActorLocationAndRotation` (* (`KismetMathLibrary.Normal` (`KismetMathLibrary.GetForwardVector` _returnvalue)) (`self.DistanceFromScene`)) _returnvalue)
  (`self.Lock Hide/Unhide`)
  (`self.updateSort`))

(fn `UserConstructionScript`)