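; 1PTable is an interactable table that the player can knock away once, after which it disappears.
; A sphere collider tracks whether PlayerBP is in range, showing an interact prompt on entry and removing all widgets on exit.
; The player's interact event, bound on BeginPlay, enables physics on TableFB and applies an acceleration rotated by the inverse actor transform.
; The actor destroys itself after a short delay.
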(event `self.SphereCollider.OnComponentBeginOverlap`
  (params (OverlappedComponent :type "PrimitiveComponent Object Reference") (OtherActor :type "Actor Object Reference") (OtherComp :type "PrimitiveComponent Object Reference") (OtherBodyIndex :type Integer) (bFromSweep :type Boolean) (SweepResult :type "HitResult Structure (by ref)"))
  ;[1 1 1] Interaction Prompt Display Based On Proximity
  (cast `/Game/Blueprints/PlayerBP` OtherActor)
  (set `self.PlayerInRange` true)
  (bind _returnvalue (`|CreateWidget` "/Game/Blueprints/Interact_prompt.Interact_prompt_C"))
  (`UserWidget.AddToViewport` _returnvalue 0))

(event `self.SphereCollider.OnComponentEndOverlap`
  (params (OverlappedComponent :type "PrimitiveComponent Object Reference") (OtherActor :type "Actor Object Reference") (OtherComp :type "PrimitiveComponent Object Reference") (OtherBodyIndex :type Integer))
  ;[1 1 1] Interaction Prompt Display Based On Proximity
  (cast `/Game/Blueprints/PlayerBP` OtherActor)
  (set `self.PlayerInRange` false)
  (`WidgetLayoutLibrary.RemoveAllWidgets`))

(event `self.ReceiveBeginPlay`
  (add `/Game/Blueprints/PlayerBP.InteractEvent` (`self.Player`) (delegate `HandleInteraction`)))

(event `HandleInteraction`
  (bind _tablefb (`self.TableFB`))
  ;[1 1 1] Interaction Code Body
  (if (`self.PlayerInRange`)
    (`PrimitiveComponent.SetSimulatePhysics` _tablefb true)
    (set `self.Used` true)
    (`PrimitiveComponent.AddForce` _tablefb (`KismetMathLibrary.Quat_RotateVector` (`KismetMathLibrary.Matrix_ToQuat` (`KismetMathLibrary.Matrix_GetInverse` (`KismetMathLibrary.Conv_TransformToMatrix` (`self.GetTransform`)))) (`KismetMathLibrary.MakeVector` -50.0)) "None" true)
    (`KismetSystemLibrary.Delay` 2.0)
    (`self.K2_DestroyActor`)))

(fn `UserConstructionScript`)