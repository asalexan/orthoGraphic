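; Child Blueprint of an interactable bottle that the player breaks with the special interact input when in range and both planes are present.
; Breaking swaps both planes' normal and highlight materials.
; Interacting again briefly shows a NewLevel widget if the player wears a glove, otherwise a dialog.
; Capsule overlaps toggle highlighting, notify the player, and manage break, collect-shard or, for single-plane objects matching the held item, completion prompts.
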(event `self.ReceiveBeginPlay`
  (`parent.ReceiveBeginPlay`)
  (add `/Game/Blueprints/PlayerBP.SpecialInteract` (`self.Player`) (delegate `Break Bottle`)))

(event `Break Bottle`
  (bind _breakbottleprompt (`self.breakBottlePrompt`))
  (if (and (`self.PlayerInRange`) (== (`self.NumPlanes`) 2))
    (if (`self.bottleBroken`)
      (if (`/Game/Blueprints/PlayerBP.wearingGlove` (`self.Player`))
        (bind _returnvalue (`|CreateWidget` "/Game/Blueprints/UI/NewLevel.NewLevel_C"))
        (`UserWidget.AddToViewport` _returnvalue 0)
        (`KismetSystemLibrary.Delay` 4.0)
        (`Widget.RemoveFromParent` _returnvalue)
        (else
          (bind _returnvalue_2 (`|CreateWidget` "/Game/Blueprints/UI/Dialog_OW.Dialog_OW_C"))
          (`UserWidget.AddToViewport` _returnvalue_2 0)
          (`KismetSystemLibrary.Delay` 4.0)
          (`Widget.RemoveFromParent` _returnvalue_2)))
      (else
        (`PrimitiveComponent.SetMaterial` (`self.Plane1`) 0 "/Game/Materials/bottlebrokenMat.bottlebrokenMat")
        (`PrimitiveComponent.SetMaterial` (`self.Plane2`) 0 "/Game/Materials/bottlebrokenMat.bottlebrokenMat")
        (set `self.plane1_mat` "/Game/Materials/bottlebrokenMat.bottlebrokenMat")
        (set `self.plane2_mat` "/Game/Materials/bottlebrokenMat.bottlebrokenMat")
        (set `self.plane1_selectedMat` "/Game/Materials/bottlebroken_selected.bottlebroken_selected")
        (set `self.plane2_selectedMat` "/Game/Materials/bottlebroken_selected.bottlebroken_selected")
        (set `self.bottleBroken` true)
        (`/Engine/EditorBlueprintResources/StandardMacros.IsValid` _breakbottleprompt
          (:`Is Valid`
            (`Widget.RemoveFromParent` _breakbottleprompt)
            (set `self.breakBottlePrompt` null)))))))

(event `self.Capsule.OnComponentBeginOverlap`
  (params (OverlappedComponent :type "PrimitiveComponent Object Reference") (OtherActor :type "Actor Object Reference") (OtherComp :type "PrimitiveComponent Object Reference") (OtherBodyIndex :type Integer) (bFromSweep :type Boolean) (SweepResult :type "HitResult Structure (by ref)"))
  ;[0 0 0] Interaction Prompt Display Based On Proximity
  (if (`self.visible`)
    (cast `/Game/Blueprints/PlayerBP` OtherActor)
    (set `self.PlayerInRange` true)
    (`/Game/Blueprints/PlayerBP.AddOverlap` (`self.Player`)) ; Player handles adding the interact prompt
    (`PrimitiveComponent.SetMaterial` (`self.Plane1`) 0 (`self.plane1_selectedMat`))
    (`PrimitiveComponent.SetMaterial` (`self.Plane2`) 0 (`self.plane2_selectedMat`))
    ;[1 0.5619 0.552] Allow player to finish object if same type as held
    (if (and (== (`self.NumPlanes`) 1) (== (`self.Label`) (`/Game/Blueprints/PlayerBP.HeldItemLabel` (`self.Player`))))
      (`/Engine/EditorBlueprintResources/StandardMacros.IsValid` (`self.CompleteObjPrompt`)
        (:`Is Valid`
          _)
        (:`Is Not Valid`
          (bind _returnvalue (`|CreateWidget` "/Game/Blueprints/UI/Complete_prompt.Complete_prompt_C"))
          (`UserWidget.AddToViewport` _returnvalue 0)
          (set `self.CompleteObjPrompt` _returnvalue))))
    ;[1 1 1] Bottle UI
    (if (== (`self.NumPlanes`) 2)
      (if (`self.bottleBroken`)
        (`/Engine/EditorBlueprintResources/StandardMacros.IsValid` (`self.collectShardPrompt`)
          (:`Is Not Valid`
            (bind _returnvalue_2 (`|CreateWidget` "/Game/Blueprints/UI/collectShardPrompt.collectShardPrompt_C"))
            (`UserWidget.AddToViewport` _returnvalue_2 0)
            (set `self.collectShardPrompt` _returnvalue_2)))
        (else
          (`/Engine/EditorBlueprintResources/StandardMacros.IsValid` (`self.breakBottlePrompt`)
            (:`Is Not Valid`
              (bind _returnvalue_3 (`|CreateWidget` "/Game/Blueprints/UI/Breakbottle_prompt.Breakbottle_prompt_C"))
              (`UserWidget.AddToViewport` _returnvalue_3 0)
              (set `self.breakBottlePrompt` _returnvalue_3))))))))

(event `self.Capsule.OnComponentEndOverlap`
  (params (OverlappedComponent :type "PrimitiveComponent Object Reference") (OtherActor :type "Actor Object Reference") (OtherComp :type "PrimitiveComponent Object Reference") (OtherBodyIndex :type Integer))
  (bind _breakbottleprompt (`self.breakBottlePrompt`))
  (bind _collectshardprompt (`self.collectShardPrompt`))
  (bind _completeobjprompt (`self.CompleteObjPrompt`))
  ;[0 0 0] Interaction Prompt Display Based On Proximity
  (cast `/Game/Blueprints/PlayerBP` OtherActor)
  (set `self.PlayerInRange` false)
  (`/Game/Blueprints/PlayerBP.SubtractOverlap` (`self.Player`)) ; Player handles removing interact prompt
  (`PrimitiveComponent.SetMaterial` (`self.Plane1`) 0 (`self.plane1_mat`))
  (`PrimitiveComponent.SetMaterial` (`self.Plane2`) 0 (`self.plane2_mat`))
  ;[1 0.5619 0.552] Allow player to finish object if same type as held
  (`/Engine/EditorBlueprintResources/StandardMacros.IsValid` _completeobjprompt
    (:`Is Valid`
      (`Widget.RemoveFromParent` _completeobjprompt)
      (set `self.CompleteObjPrompt` null))
    (:`Is Not Valid`
      _))
  ;[1 1 1] Bottle UI
  (`/Engine/EditorBlueprintResources/StandardMacros.IsValid` _collectshardprompt
    (:`Is Valid`
      (`Widget.RemoveFromParent` _collectshardprompt)
      (set `self.collectShardPrompt` null))
    (:`Is Not Valid`
      _))
  (`/Engine/EditorBlueprintResources/StandardMacros.IsValid` _breakbottleprompt
    (:`Is Valid`
      (`Widget.RemoveFromParent` _breakbottleprompt)
      (set `self.breakBottlePrompt` null))))

(fn `UserConstructionScript`
  (`parent.UserConstructionScript`))