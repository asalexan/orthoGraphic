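; SceneObjectBP is an interactable scene object that reacts to the player's interact event while the player is in range.
; ColliderPlane1 overlaps with PlayerBP set the range flag and show the prompt widget, removing all widgets on exit.
; HandleInteraction, bound on BeginPlay, branches on NumPlanes: one plane gets physics and a push before delayed destruction, two planes yaw the actor a quarter turn.
; The collider scale setup is never called.
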(event `HandleInteraction`
  (bind _colliderplane1 (`self.ColliderPlane1`))
  (if (and (`self.PlayerInRange`) (== (`self.NumPlanes`) 1))
    (`PrimitiveComponent.SetSimulatePhysics` _colliderplane1 true)
    (set `self.Used` true)
    (`PrimitiveComponent.AddForce` _colliderplane1 (`KismetMathLibrary.MakeVector` -100.0) "None" true)
    (`KismetSystemLibrary.Delay` 5.0)
    (`self.K2_DestroyActor`)
    (elif (and (`self.PlayerInRange`) (== (`self.NumPlanes`) 2))
      (`self.K2_AddActorLocalRotation` (`KismetMathLibrary.MakeRotator` 0.0 0.0 90.0)))))

(event `self.ReceiveBeginPlay`
  (add `/Game/Blueprints/PlayerBP.InteractEvent` (`self.Player`) (delegate `HandleInteraction`)))

(event `self.ColliderPlane1.OnComponentBeginOverlap`
  (params (OverlappedComponent :type "PrimitiveComponent Object Reference") (OtherActor :type "Actor Object Reference") (OtherComp :type "PrimitiveComponent Object Reference") (OtherBodyIndex :type Integer) (bFromSweep :type Boolean) (SweepResult :type "HitResult Structure (by ref)"))
  ;[0 0 0] Interaction Prompt Display Based On Proximity
  (cast `/Game/Blueprints/PlayerBP` OtherActor)
  (set `self.PlayerInRange` true)
  (bind _returnvalue (`|CreateWidget` "/Game/Blueprints/Interact_prompt.Interact_prompt_C"))
  (`UserWidget.AddToViewport` _returnvalue 0))

(event `self.ColliderPlane1.OnComponentEndOverlap`
  (params (OverlappedComponent :type "PrimitiveComponent Object Reference") (OtherActor :type "Actor Object Reference") (OtherComp :type "PrimitiveComponent Object Reference") (OtherBodyIndex :type Integer))
  ;[0 0 0] Interaction Prompt Display Based On Proximity
  (cast `/Game/Blueprints/PlayerBP` OtherActor)
  (set `self.PlayerInRange` false)
  (`WidgetLayoutLibrary.RemoveAllWidgets`))

(fn `UserConstructionScript`)