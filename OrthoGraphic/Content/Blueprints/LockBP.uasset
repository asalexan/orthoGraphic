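; LockBP is a lock actor that shows or hides its cube according to the orthographic camera's orientation.
; On BeginPlay it binds to the camera's lock hide/unhide dispatcher, avoiding Tick.
; When fired, it compares the camera root's forward vector to its View vector within a small tolerance.
; A match flattens the cube's Z scale to zero unless Locked is set; otherwise full scale is restored.
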(event `self.ReceiveBeginPlay`
  ;[0 0 0] Bind Hide/Unhide Lock Event (triggered by OrthoCamera input)
  (add `/Game/Blueprints/OrthoCamera.Lock Hide/Unhide` (`self.Camera`) (delegate `Lock Hide/Unhide`)))

(event `Lock Hide/Unhide`
  ;[0 0 0] Hide/Unhide Lock Event
  (if (== (`KismetMathLibrary.GetForwardVector` (`SceneComponent.K2_GetComponentRotation` (`Actor.RootComponent` (`self.Camera`)))) (`self.View`))
    (if (not (`self.Locked`))
      (`SceneComponent.SetWorldScale3D` (`self.Cube`) (1.8 0.05 0.0)) ; Hide lock if looking down matching axis
    )
    (else
      (`SceneComponent.SetWorldScale3D` (`self.Cube`) (1.8 0.05 0.9)) ; Show lock if not looking down matching axis
    )))

(fn `UserConstructionScript`)