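; Child Blueprint of a knife that a button lifts, apparently as part of a magnet puzzle with a fan.
; It binds to the button's toggle event and snaps to a hardcoded start position on BeginPlay.
; Timelines drive Lerped location offsets: up when the button is on and the knife is in magnet range, otherwise straight down.
; If the fan is on during descent, the knife also shifts sideways along Y and leaves magnet range.
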(event `ButtonToggled`
  (bind _startingpos (`self.startingPos`))
  (if (and (`/Game/Blueprints/buttonChild.buttonOn` (`self.Button`)) (`self.inMagRange`))
    (bind (_direction _floatoutput) (`Timeline|Timeline_0` :!via `PlayFromStart`)
      (:`Update`
        (`self.K2_SetActorLocation` (+ _startingpos (`KismetMathLibrary.MakeVector` 0.0 0.0 (`KismetMathLibrary.Lerp` 0.0 115.68 _floatoutput))))))
    (elif (`/Game/Blueprints/fanChild.fanOn` (`self.Fan`))
      (bind (_direction_2 _floatoutput_2) (`Timeline|Timeline_2` :!via `PlayFromStart`)
        (:`Update`
          (`self.K2_SetActorLocation` (- (+ _startingpos (0.0 0.0 115.68)) (`KismetMathLibrary.MakeVector` 0.0 (`KismetMathLibrary.Lerp` 0.0 -170.0 _floatoutput_2) (`KismetMathLibrary.Lerp` 0.0 115.68 _floatoutput_2))))
          (set `self.inMagRange` false)))
      (else
        (bind (_direction_3 _floatoutput_3) (`Timeline|Timeline_1` :!via `PlayFromStart`)
          (:`Update`
            (`self.K2_SetActorLocation` (- (+ _startingpos (0.0 0.0 115.68)) (`KismetMathLibrary.MakeVector` 0.0 0.0 (`KismetMathLibrary.Lerp` 0.0 115.68 _floatoutput_3))))))))))

(event `self.ReceiveBeginPlay`
  (`parent.ReceiveBeginPlay`)
  (add `/Game/Blueprints/buttonChild.ButtonToggled` (`self.Button`) (delegate `ButtonToggled`))
  (bind _output_get (set `self.startingPos` (15.78 4.66 -56.119999)))
  (`self.K2_SetActorLocation` _output_get))

(event `self.ReceiveTick`
  (params (DeltaSeconds :type "Float (single-precision)")))

(fn `UserConstructionScript`
  (`parent.UserConstructionScript`))