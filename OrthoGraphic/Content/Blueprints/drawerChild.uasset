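; Searchable drawer, a child Blueprint that can hand the player an item when they press special interact in range.
; Overlap adds or removes the search prompt; searching requires NumPlanes to equal 2.
; DrawerItemLabel picks the result: Glove equips once with a material swap, Knife loads the next level, other textured items become the held item.
; Otherwise an empty-drawer message shows; pop-up widgets use timed delays.
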(event `self.ReceiveBeginPlay`
  (`parent.ReceiveBeginPlay`)
  (add `/Game/Blueprints/PlayerBP.SpecialInteract` (`self.Player`) (delegate `Check Drawer`)))

(event `Check Drawer`
  (bind _player (`self.Player`))
  (if (and (`self.PlayerInRange`) (== (`self.NumPlanes`) 2))
    (if (== (`self.DrawerItemLabel`) "Glove")
      (if (not (`self.itemRetrieved`))
        (bind _returnvalue (`|CreateWidget` "/Game/Blueprints/UI/foundAGlove.foundAGlove_C"))
        (`UserWidget.AddToViewport` _returnvalue 0)
        (set `/Game/Blueprints/PlayerBP.wearingGlove` true (`self.Player`))
        (set `self.itemRetrieved` true)
        (`PrimitiveComponent.SetMaterial` (`/Game/Blueprints/PlayerBP.StaticMesh` (`self.Player`)) 0 "/Game/Materials/playerWGlove.playerWGlove")
        (`KismetSystemLibrary.Delay` 4.0)
        (`Widget.RemoveFromParent` _returnvalue))
      (else
        (`/Engine/EditorBlueprintResources/StandardMacros.IsValid` (`self.DrawerItemTexture`)
          (:`Is Valid`
            (if (== (`self.DrawerItemLabel`) "Knife")
              (bind _returnvalue_2 (`|CreateWidget` "/Game/Blueprints/UI/NewLevel.NewLevel_C"))
              (`UserWidget.AddToViewport` _returnvalue_2 0)
              (`KismetSystemLibrary.Delay` 4.0)
              (`/Game/Blueprints/PlayerBP.LoadNextLevel` (`self.Player`))
              (else
                (set `/Game/Blueprints/PlayerBP.HeldItemLabel` (`self.DrawerItemLabel`) _player)
                (`Image.SetBrushFromTexture` (`/Game/Blueprints/UI/HeldItemUI.HeldItemImg` (`/Game/Blueprints/PlayerBP.heldItemWidget` _player)) (`self.DrawerItemTexture`) false))))
          (:`Is Not Valid`
            (bind _returnvalue_3 (`|CreateWidget` "/Game/Blueprints/UI/EmptyDrawer.EmptyDrawer_C"))
            (`UserWidget.AddToViewport` _returnvalue_3 0)
            (`KismetSystemLibrary.Delay` 5.0)
            (`Widget.RemoveFromParent` _returnvalue_3)))))))

(event `self.Capsule.OnComponentBeginOverlap`
  (params (OverlappedComponent :type "PrimitiveComponent Object Reference") (OtherActor :type "Actor Object Reference") (OtherComp :type "PrimitiveComponent Object Reference") (OtherBodyIndex :type Integer) (bFromSweep :type Boolean) (SweepResult :type "HitResult Structure (by ref)"))
  ;[0 0 0] Interaction Prompt Display Based On Proximity
  (`self.Parent Begin Overlap` OtherActor)
  ;[1 1 1] Drawer UI
  (if (and (== (`self.NumPlanes`) 2) (not (`self.itemRetrieved`)))
    (bind _returnvalue (`self.Create Special Interact Prompt` (`self.searchDrawerPrompt`) "Press I to Search Drawer"))
    (set `self.searchDrawerPrompt` _returnvalue)))

(event `self.Capsule.OnComponentEndOverlap`
  (params (OverlappedComponent :type "PrimitiveComponent Object Reference") (OtherActor :type "Actor Object Reference") (OtherComp :type "PrimitiveComponent Object Reference") (OtherBodyIndex :type Integer))
  ;[0 0 0] Interaction Prompt Display Based On Proximity
  (`self.Parent End Overlap` OtherActor)
  ;[1 1 1] Drawer UI
  (`self.Delete Special Interact Prompt` (`self.searchDrawerPrompt`))
  (set `self.searchDrawerPrompt` null))

(fn `UserConstructionScript`
  (`parent.UserConstructionScript`))