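; Interactive one- or two-plane scene object for a rotating-camera world, highlighted and reacting to player events when in range.
; Forward-vector tests against the camera's viewing axis choose which collider blocks after view spins.
; Interacting topples a camera-aligned single plane for collection and delayed destruction, or yaws a two-plane object 90°; a matching held item restores the second plane.
; Camera-driven events set translucent sort priority from position along the viewing axis.
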(event `self.ReceiveBeginPlay`
  (bind _player (`self.Player`))
  (bind _player_2 (`self.Player`))
  (bind _colliderplane2 (`self.ColliderPlane2`))
  (bind _colliderplane1 (`self.ColliderPlane1`))
  (add `/Game/Blueprints/OrthoCamera.updateSort` (`self.camera`) (delegate `updateSort_Event`))
  (add `/Game/Blueprints/PlayerBP.CollectItemEvent` _player_2 (delegate `Collect Item`))
  (add `/Game/Blueprints/PlayerBP.CompleteObjEvent` _player_2 (delegate `CompleteObjEvent`))
  (`PrimitiveComponent.SetCollisionResponseToAllChannels` (`self.ColliderPlane1`) "ECR_Overlap")
  (`PrimitiveComponent.SetCollisionResponseToAllChannels` (`self.ColliderPlane2`) "ECR_Overlap")
  (`PrimitiveComponent.SetCollisionResponseToAllChannels` (`self.Plane1`) "ECR_Overlap")
  (`PrimitiveComponent.SetCollisionResponseToAllChannels` (`self.Plane2`) "ECR_Overlap")
  (bind _output_get (set `self.visible` (`KismetMathLibrary.NearlyEqual_FloatFloat` (`KismetMathLibrary.VSize` (`KismetMathLibrary.Normal` (`KismetMathLibrary.Cross_VectorVector` (`KismetMathLibrary.GetForwardVector` (.rotation (`SceneComponent.K2_GetComponentToWorld` _colliderplane1))) (`/Game/Blueprints/OrthoCamera.ViewingAxis` (`self.camera`))))))))
  (if _output_get
    (`PrimitiveComponent.SetCollisionResponseToAllChannels` _colliderplane1 "ECR_Block")
    (`PrimitiveComponent.SetCollisionResponseToAllChannels` _colliderplane2 "ECR_Overlap")
    (else
      (`PrimitiveComponent.SetCollisionResponseToAllChannels` _colliderplane1 "ECR_Overlap")
      (`PrimitiveComponent.SetCollisionResponseToAllChannels` _colliderplane2 "ECR_Block")))
  (if (== (`self.NumPlanes`) 1)
    (`PrimitiveComponent.SetCollisionResponseToAllChannels` (`self.ColliderPlane2`) "ECR_Overlap"))
  (add `/Game/Blueprints/PlayerBP.SpinViewLeft` _player (delegate `UpdateCollisions`))
  (add `/Game/Blueprints/PlayerBP.SpinViewRight` _player (delegate `UpdateCollisions`))
  (add `/Game/Blueprints/PlayerBP.InteractEvent` (`self.Player`) (delegate `HandleInteraction`)))

(event `HandleInteraction`
  (bind _colliderplane2 (`self.ColliderPlane2`))
  (bind _completeobjprompt (`self.CompleteObjPrompt`))
  (bind _colliderplane1 (`self.ColliderPlane1`))
  (bind _returnvalue (`KismetMathLibrary.MakeRotator` 0.0 (`self.angle`)))
  (bind _returnvalue_2 (`self.K2_GetActorLocation` (`self.camera`)))
  (bind _returnvalue_3 (`KismetMathLibrary.Dot_VectorVector` (`KismetMathLibrary.GetForwardVector` (.rotation (`SceneComponent.K2_GetComponentToWorld` _colliderplane1))) (`/Game/Blueprints/OrthoCamera.ViewingAxis` (`self.camera`))))
  (if (and (and (`self.PlayerInRange`) (== (`self.NumPlanes`) 1)) (`KismetMathLibrary.NearlyEqual_FloatFloat` (`KismetMathLibrary.VSize` (`KismetMathLibrary.Normal` (`KismetMathLibrary.Cross_VectorVector` (`/Game/Blueprints/OrthoCamera.ViewingAxis` (`self.camera`)) (`KismetMathLibrary.GetAxes` (`self.K2_GetActorRotation`)))))))
    (if (>= (`KismetMathLibrary.Vector_Distance` _returnvalue_2 (`SceneComponent.K2_GetComponentLocation` (`self.Scene`))) (`KismetMathLibrary.Vector_Distance` _returnvalue_2 (`self.K2_GetActorLocation` (`self.Player`))))
      (set `self.angle` 25.0)
      (else
        (set `self.angle` -25.0)))
    (if (== (`KismetMathLibrary.Vector_GetAbs` (`KismetMathLibrary.Normal` (`/Game/Blueprints/OrthoCamera.ViewingAxis` (`self.camera`)))) (1.0 0.0 0.0))
      (`self.K2_AddActorLocalRotation` _returnvalue)
      (else
        (`self.K2_AddActorLocalRotation` _returnvalue)))
    (`KismetSystemLibrary.Delay` 0.2)
    (`PrimitiveComponent.SetCollisionEnabled` (`self.ColliderPlane2`) "NoCollision")
    (`PrimitiveComponent.SetSimulatePhysics` (`self.ColliderPlane1`) true)
    (set `self.visible` false)
    (set `self.used` true)
    (`/Game/Blueprints/PlayerBP.SubtractOverlap` (`self.Player`))
    (`/Engine/EditorBlueprintResources/StandardMacros.IsValid` _completeobjprompt
      (:`Is Valid`
        (`Widget.RemoveFromParent` _completeobjprompt)
        (set `self.CompleteObjPrompt` null))
      (:`Is Not Valid`
        _))
    (bind _returnvalue_4 (`|CreateWidget` "/Game/Blueprints/UI/Collect_prompt.Collect_prompt_C"))
    (`UserWidget.AddToViewport` _returnvalue_4 0)
    (bind _output_get (set `self.CollectPrompt` _returnvalue_4))
    (`KismetSystemLibrary.Delay` 5.0)
    (`self.K2_DestroyActor`)
    (`/Engine/EditorBlueprintResources/StandardMacros.IsValid` _output_get
      (:`Is Valid`
        (`Widget.RemoveFromParent` _output_get)))
    (elif (and (`self.PlayerInRange`) (== (`self.NumPlanes`) 2))
      (`self.K2_AddActorLocalRotation` (`KismetMathLibrary.MakeRotator` 0.0 0.0 90.0))
      (if (and (>= _returnvalue_3 -1e-05) (<= _returnvalue_3 1e-05))
        (`PrimitiveComponent.SetCollisionResponseToAllChannels` _colliderplane1 "ECR_Overlap")
        (`PrimitiveComponent.SetCollisionResponseToAllChannels` _colliderplane2 "ECR_Block")
        (else
          (`PrimitiveComponent.SetCollisionResponseToAllChannels` _colliderplane1 "ECR_Block")
          (`PrimitiveComponent.SetCollisionResponseToAllChannels` _colliderplane2 "ECR_Overlap"))))))

(event `UpdateCollisions`
  (bind _colliderplane2 (`self.ColliderPlane2`))
  (bind _colliderplane1 (`self.ColliderPlane1`))
  (bind _output_get (set `self.visible` (`KismetMathLibrary.NearlyEqual_FloatFloat` (`KismetMathLibrary.VSize` (`KismetMathLibrary.Normal` (`KismetMathLibrary.Cross_VectorVector` (`KismetMathLibrary.GetForwardVector` (.rotation (`SceneComponent.K2_GetComponentToWorld` _colliderplane1))) (`/Game/Blueprints/OrthoCamera.ViewingAxis` (`self.camera`))))))))
  (if _output_get
    (`PrimitiveComponent.SetCollisionResponseToAllChannels` _colliderplane1 "ECR_Block")
    (`PrimitiveComponent.SetCollisionResponseToAllChannels` _colliderplane2 "ECR_Overlap")
    (else
      (`PrimitiveComponent.SetCollisionResponseToAllChannels` _colliderplane1 "ECR_Overlap")
      (`PrimitiveComponent.SetCollisionResponseToAllChannels` _colliderplane2 "ECR_Block")))
  (if (== (`self.NumPlanes`) 1)
    (`PrimitiveComponent.SetCollisionResponseToAllChannels` (`self.ColliderPlane2`) "ECR_Overlap")))

(event `updateSort_Event`
  (bind _returnvalue (`KismetMathLibrary.FTrunc` (* (+ (.x (* (`SceneComponent.K2_GetComponentLocation` (`self.Scene`)) (`/Game/Blueprints/OrthoCamera.ViewingAxis` (`self.camera`)))) (.y (* (`SceneComponent.K2_GetComponentLocation` (`self.Scene`)) (`/Game/Blueprints/OrthoCamera.ViewingAxis` (`self.camera`)))) (.z (* (`SceneComponent.K2_GetComponentLocation` (`self.Scene`)) (`/Game/Blueprints/OrthoCamera.ViewingAxis` (`self.camera`))))) -1.0)))
  (`PrimitiveComponent.SetTranslucentSortPriority` (`self.Plane1`) _returnvalue)
  (`PrimitiveComponent.SetTranslucentSortPriority` (`self.Plane2`) _returnvalue))

(event `Collect Item`
  (if (`self.used`)
    (set `/Game/Blueprints/PlayerBP.HeldItemTemp` self (`self.Player`))))

(event `CompleteObjEvent`
  (bind _completeobjprompt (`self.CompleteObjPrompt`))
  (if (and (== (`self.NumPlanes`) 1) (== (`self.Label`) (`/Game/Blueprints/PlayerBP.HeldItemLabel` (`self.Player`))) (`self.PlayerInRange`))
    (set `self.NumPlanes` 2)
    (`SceneComponent.SetHiddenInGame` (`self.Plane2`) false false)
    (`PrimitiveComponent.SetMaterial` (`self.Plane2`) 0 (`self.plane2_mat`))
    (`/Engine/EditorBlueprintResources/StandardMacros.IsValid` _completeobjprompt
      (:`Is Valid`
        (`Widget.RemoveFromParent` _completeobjprompt)))))

(event `self.Capsule.OnComponentBeginOverlap`
  (params (OverlappedComponent :type "PrimitiveComponent Object Reference") (OtherActor :type "Actor Object Reference") (OtherComp :type "PrimitiveComponent Object Reference") (OtherBodyIndex :type Integer) (bFromSweep :type Boolean) (SweepResult :type "HitResult Structure (by ref)"))
  ;[0 0 0] Interaction Prompt Display Based On Proximity
  (if (`self.visible`)
    (cast `/Game/Blueprints/PlayerBP` OtherActor)
    (set `self.PlayerInRange` true)
    (`/Game/Blueprints/PlayerBP.AddOverlap` (`self.Player`)) ; Player handles adding the interact prompt
    (`PrimitiveComponent.SetMaterial` (`self.Plane1`) 0 (`self.plane1_selectedMat`))
    (`PrimitiveComponent.SetMaterial` (`self.Plane2`) 0 (`self.plane2_selectedMat`))
    ;[1 0.5619 0.552] Allow player to finish object if same type as held
    (if (and (== (`self.NumPlanes`) 1) (== (`self.Label`) (`/Game/Blueprints/PlayerBP.HeldItemLabel` (`self.Player`))))
      (`/Engine/EditorBlueprintResources/StandardMacros.IsValid` (`self.CompleteObjPrompt`)
        (:`Is Not Valid`
          (bind _returnvalue (`|CreateWidget` "/Game/Blueprints/UI/Complete_prompt.Complete_prompt_C"))
          (`UserWidget.AddToViewport` _returnvalue 0)
          (set `self.CompleteObjPrompt` _returnvalue))))))

(event `self.Capsule.OnComponentEndOverlap`
  (params (OverlappedComponent :type "PrimitiveComponent Object Reference") (OtherActor :type "Actor Object Reference") (OtherComp :type "PrimitiveComponent Object Reference") (OtherBodyIndex :type Integer))
  (bind _completeobjprompt (`self.CompleteObjPrompt`))
  ;[0 0 0] Interaction Prompt Display Based On Proximity
  (cast `/Game/Blueprints/PlayerBP` OtherActor)
  (set `self.PlayerInRange` false)
  (`/Game/Blueprints/PlayerBP.SubtractOverlap` (`self.Player`)) ; Player handles removing interact prompt
  (`PrimitiveComponent.SetMaterial` (`self.Plane1`) 0 (`self.plane1_mat`))
  (`PrimitiveComponent.SetMaterial` (`self.Plane2`) 0 (`self.plane2_mat`))
  ;[1 0.5619 0.552] Allow player to finish object if same type as held
  (`/Engine/EditorBlueprintResources/StandardMacros.IsValid` _completeobjprompt
    (:`Is Valid`
      (`Widget.RemoveFromParent` _completeobjprompt)
      (set `self.CompleteObjPrompt` null))))

(fn `UserConstructionScript`)