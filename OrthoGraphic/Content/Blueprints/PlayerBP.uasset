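; Player Blueprint that handles camera-relative walking and relays interact and view-spin input.
; Enter and the Spin Left/Right actions fire event dispatchers for other objects to handle.
; Walk Side and Walk Back axes offset the actor's location along camera vectors each frame, without sweep or delta-time scaling.
; Both also set facing from camera yaw offsets, with a walkBack flag gating the reset to camera rotation when sideways input stops.
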(event `Key|Enter`
  (params (Key :type "Key Structure"))
  (:`Pressed`
    (`self.InteractEvent`)))

(event `InputAction|Spin Left`
  (params (Key :type "Key Structure"))
  ;[0 0 0] Bind camera actions
  (:`Pressed`
    (`self.SpinViewLeft`)))

(event `InputAction|Spin Right`
  (params (Key :type "Key Structure"))
  ;[0 0 0] Bind camera actions
  (:`Pressed`
    (`self.SpinViewRight`)))

(event `InputAxis|Walk Side`
  (params (AxisValue :type "Float (single-precision)"))
  (`self.K2_SetActorLocation` (+ (* (`KismetMathLibrary.GetRightVector` (`self.K2_GetActorRotation` (`self.Camera`))) (* AxisValue 0.5)) (`self.K2_GetActorLocation`)))
  (if (> (`KismetMathLibrary.Abs` AxisValue) 0.0)
    (`self.K2_SetActorRotation` (`KismetMathLibrary.Conv_VectorToRotator` (`KismetMathLibrary.RotateAngleAxis` (`KismetMathLibrary.Conv_RotatorToVector` (`self.K2_GetActorRotation` (`self.Camera`))) 90.0 (0.0 0.0 1.0))))
    (else
      ;[0 0 0] If no input, face forward
      (if (not (> (stale `InputAxis|Walk Back` AxisValue) 0.0))
        (`self.K2_SetActorRotation` (`self.K2_GetActorRotation` (`self.Camera`)))))))

(event `InputAxis|Walk Back`
  (params (AxisValue :type "Float (single-precision)"))
  (`self.K2_SetActorLocation` (+ (* (`KismetMathLibrary.GetForwardVector` (`self.K2_GetActorRotation` (`self.Camera`))) (* AxisValue 0.5)) (`self.K2_GetActorLocation`)))
  (if (> AxisValue 0.0)
    (`self.K2_SetActorRotation` (`KismetMathLibrary.Conv_VectorToRotator` (`KismetMathLibrary.RotateAngleAxis` (`KismetMathLibrary.Conv_RotatorToVector` (`self.K2_GetActorRotation` (`self.Camera`))) 180.0 (0.0 0.0 1.0))))))

(fn `UserConstructionScript`)