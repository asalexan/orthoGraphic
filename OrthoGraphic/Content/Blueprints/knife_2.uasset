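; Collectible knife that, when picked up, unlocks the level lock at the current level index and advances that index.
; A sphere collider tracks player proximity, showing an interaction prompt and swapping the knife to a selected material.
; The player's pickup event increments the knife count, hides the mesh, disables collision and shows a new-level widget for three seconds.
; UI changes clear all widgets and recreate the base widget.
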(event `self.ReceiveBeginPlay`
  (bind _returnvalue (`|CreateWidget` "/Game/Blueprints/UI/NewWidgetBlueprint.NewWidgetBlueprint_C"))
  (`UserWidget.AddToViewport` _returnvalue 0)
  (add `/Game/Blueprints/PlayerBP.PickUpKnifeEvent` (`self.Player`) (delegate `knifeInteraction`)))

(event `knifeInteraction`
  ;[1 1 1] Collect Knife
  (if (`self.Player_Near`)
    _
    (else
      _))
  (set `self.knifeNum` (+ (`self.knifeNum`) 1))
  (`SceneComponent.SetVisibility` (`self.knife`) false false)
  (`PrimitiveComponent.SetCollisionEnabled` (`self.SphereCollider`) "NoCollision")
  (bind _returnvalue (`|CreateWidget` "/Game/Blueprints/UI/NewLevel.NewLevel_C"))
  (`UserWidget.AddToViewport` _returnvalue 0)
  (`KismetSystemLibrary.Delay` 3.0)
  (`WidgetLayoutLibrary.RemoveAllWidgets`)
  (bind _returnvalue_2 (`|CreateWidget` "/Game/Blueprints/UI/NewWidgetBlueprint.NewWidgetBlueprint_C"))
  (`UserWidget.AddToViewport` _returnvalue_2 0)
  (bind _outactors (`GameplayStatics.GetAllActorsOfClass` "/Game/Blueprints/LockBP.LockBP_C"))
  (set `/Game/Blueprints/LockBP.Locked` false (`|GetArrayItem` _outactors (`self.currLevel`)))
  (set `self.currLevel` (+ (`self.currLevel`) 1)))

(event `self.SphereCollider.OnComponentBeginOverlap`
  (params (OverlappedComponent :type "PrimitiveComponent Object Reference") (OtherActor :type "Actor Object Reference") (OtherComp :type "PrimitiveComponent Object Reference") (OtherBodyIndex :type Integer) (bFromSweep :type Boolean) (SweepResult :type "HitResult Structure (by ref)"))
  ;[1 1 1] Interaction Prompt Display Based On Proximity
  (cast `/Game/Blueprints/PlayerBP` OtherActor)
  (set `self.Player_Near` true)
  (bind _returnvalue (`|CreateWidget` "/Game/Blueprints/UI/knife_interaction.knife_interaction_C"))
  (`UserWidget.AddToViewport` _returnvalue 0)
  (`PrimitiveComponent.SetMaterial` (`self.knife`) 0 (`self.knife_selectedMat`)))

(event `self.SphereCollider.OnComponentEndOverlap`
  (params (OverlappedComponent :type "PrimitiveComponent Object Reference") (OtherActor :type "Actor Object Reference") (OtherComp :type "PrimitiveComponent Object Reference") (OtherBodyIndex :type Integer))
  ;[1 1 1] Interaction Prompt Display Based On Proximity
  (cast `/Game/Blueprints/PlayerBP` OtherActor)
  (set `self.Player_Near` false)
  (`WidgetLayoutLibrary.RemoveAllWidgets`)
  (bind _returnvalue (`|CreateWidget` "/Game/Blueprints/UI/NewWidgetBlueprint.NewWidgetBlueprint_C"))
  (`UserWidget.AddToViewport` _returnvalue 0))

(fn `UserConstructionScript`)